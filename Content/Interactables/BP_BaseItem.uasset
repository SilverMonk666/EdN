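; BP_BaseItem is a base item actor that can be picked up through an Interaction event.
; On interaction, it checks whether the instigator has inventory space, passes its ItemInfo struct via PickUpMessage, then destroys itself.
; The construction script writes the actor's own class into ItemInfo while keeping the other fields, so the pickup data records which class it came from.
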(event `/Game/Interactables/BP_interact.Interaction`
  (params (Instigator :type "/Game/Characters/MyCharacter/CH_MyCharacter Object Reference"))
  (if (`/Game/Characters/MyCharacter/CH_MyCharacter.HasSpaceInInventory` Instigator)
    (message `/Game/Interactables/BP_interact.PickUp` Instigator (`self.ItemInfo`))
    (`self.K2_DestroyActor`)))

(fn `UserConstructionScript`
  (bind (_iteminfo_itemtype _iteminfo_itemname _iteminfo_itemimage _iteminfo_itemclass _iteminfo_itemindex _iteminfo_itemslot _iteminfo_itemvalue) (break `/Game/Interactables/FItemInfo` (`self.ItemInfo`)))
  (`parent.UserConstructionScript`)
  (set `self.ItemInfo` (make `/Game/Interactables/FItemInfo` _iteminfo_itemtype _iteminfo_itemname _iteminfo_itemimage (`GameplayStatics.GetObjectClass` self) _iteminfo_itemindex _iteminfo_itemslot _iteminfo_itemvalue)))