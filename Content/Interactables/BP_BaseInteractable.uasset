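; BP_BaseInteractable is a base interactable that highlights itself while the player character is within range.
; Overlapping InteractableArea registers it with CH_MyCharacter and swaps the mesh's first material to Highlight.
; Ending the overlap unregisters it and restores the material cached at BeginPlay.
; SetHighlight is an empty stub, with unconnected custom-depth and material nodes left unused.
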(event `self.ReceiveBeginPlay`
  (set `self.BaseColor` (`PrimitiveComponent.GetMaterial` (`self.InteractableMesh`) 0)))

(event `self.InteractableArea.OnComponentBeginOverlap`
  (params (OverlappedComponent :type "PrimitiveComponent Object Reference") (OtherActor :type "Actor Object Reference") (OtherComp :type "PrimitiveComponent Object Reference") (OtherBodyIndex :type Integer) (bFromSweep :type Boolean) (SweepResult :type "HitResult Structure (by ref)"))
  (bind _asch_my_character (cast `/Game/Characters/MyCharacter/CH_MyCharacter` OtherActor))
  (message `/Game/Interactables/BP_interact.RegisterInteractable` _asch_my_character self)
  (`PrimitiveComponent.SetMaterial` (`self.InteractableMesh`) 0 "/Game/Materials/Highlight.Highlight"))

(event `self.InteractableArea.OnComponentEndOverlap`
  (params (OverlappedComponent :type "PrimitiveComponent Object Reference") (OtherActor :type "Actor Object Reference") (OtherComp :type "PrimitiveComponent Object Reference") (OtherBodyIndex :type Integer))
  (bind _asch_my_character (cast `/Game/Characters/MyCharacter/CH_MyCharacter` OtherActor))
  (message `/Game/Interactables/BP_interact.UnregisterInteractable` _asch_my_character self)
  (`PrimitiveComponent.SetMaterial` (`self.InteractableMesh`) 0 (`self.BaseColor`)))

(fn `SetHighlight`
  (params (`Highlight?` :type Boolean)))

(fn `UserConstructionScript`)